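; Landscape brush tool that procedurally paints weightmap layers and shapes the edges of a landscape's heightmap.
; RenderWeightmap switches on layer name, drawing a parameterized brush material for rocks, grass, gravel, grid, no-grass and optional leaves.
; The Asphalt layer calls DrawBuildings instead of using a material.
; RenderHeightmap draws a noisy edge falloff material when the falloff distance is positive.
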(event `self.RenderWeightmap`
  (params (InLayerName :type "Name (by ref)"))
  (bind _randomleavesscale (`self.RandomLeavesScale`))
  (switch `name` InLayerName
    (:`Rocks`
      (bind _returnvalue (`self.CreateMID` "/Game/BrickRigs/Dev/Tools/LandscapeBrushes/Materials/M_LandscapeRocksBrush.M_LandscapeRocksBrush"))
      (`MaterialInstanceDynamic.SetScalarParameterValue` _returnvalue "SlopeStart" (`self.RockSlopeStart`))
      (`MaterialInstanceDynamic.SetScalarParameterValue` _returnvalue "SlopeContrast" (`self.RockSlopeContrast`))
      (`self.DrawMaterial` _returnvalue))
    (:`Asphalt`
      (`self.DrawBuildings`))
    (:`NoGrass`
      (bind _returnvalue_2 (`self.CreateMID` "/Game/BrickRigs/Dev/Tools/LandscapeBrushes/Materials/M_LandscapeNoGrassBrush.M_LandscapeNoGrassBrush"))
      (`self.DrawMaterial` _returnvalue_2))
    (:`Grid`
      (bind _returnvalue_3 (`self.CreateMID` "/Game/BrickRigs/Dev/Tools/LandscapeBrushes/Materials/M_LandscapeGridBrush.M_LandscapeGridBrush"))
      (`MaterialInstanceDynamic.SetScalarParameterValue` _returnvalue_3 "GridHeight" (`self.GridHeight`))
      (`self.DrawMaterial` _returnvalue_3))
    (:`Gravel`
      (bind _returnvalue_4 (`self.CreateMID` "/Game/BrickRigs/Dev/Tools/LandscapeBrushes/Materials/M_LandscapeGravelBrush.M_LandscapeGravelBrush"))
      (`MaterialInstanceDynamic.SetScalarParameterValue` _returnvalue_4 "NoiseScale" (`self.GravelNoiseScale`))
      (`self.DrawMaterial` _returnvalue_4))
    (:`Grass`
      (bind _returnvalue_5 (`self.CreateMID` "/Game/BrickRigs/Dev/Tools/LandscapeBrushes/Materials/M_LandscapeGrassBrush.M_LandscapeGrassBrush"))
      (`MaterialInstanceDynamic.SetScalarParameterValue` _returnvalue_5 "bIsDesert" (`KismetMathLibrary.Conv_BoolToDouble` (`self.bIsDesert`)))
      (`self.DrawMaterial` _returnvalue_5))
    (:`Leaves`
      (if (> _randomleavesscale 0.0)
        (bind _returnvalue_6 (`self.CreateMID` "/Game/BrickRigs/Dev/Tools/LandscapeBrushes/Materials/M_LandscapeLeavesBrush.M_LandscapeLeavesBrush"))
        (`MaterialInstanceDynamic.SetScalarParameterValue` _returnvalue_6 "NoiseScale" _randomleavesscale)
        (`self.DrawMaterial` _returnvalue_6)))))

(event `self.RenderHeightmap`
  (if (> (`self.EdgeFalloffDistance`) 0.0)
    (bind _returnvalue (`self.CreateMID` "/Game/BrickRigs/Dev/Tools/LandscapeBrushes/Materials/M_LandscapeHeightmapBrush.M_LandscapeHeightmapBrush"))
    (`MaterialInstanceDynamic.SetScalarParameterValue` _returnvalue "FalloffDistance" (`self.EdgeFalloffDistance`))
    (`MaterialInstanceDynamic.SetScalarParameterValue` _returnvalue "FalloffBias" (`self.EdgeFalloffBias`))
    (`MaterialInstanceDynamic.SetScalarParameterValue` _returnvalue "EdgeHeight" (`self.EdgeHeight`))
    (`MaterialInstanceDynamic.SetScalarParameterValue` _returnvalue "NoiseScale" (`self.NoiseScale`))
    (`MaterialInstanceDynamic.SetScalarParameterValue` _returnvalue "SpreadDistance" (`self.NoiseSpreadDistance`))
    (`self.DrawMaterial` _returnvalue)))

(fn `UserConstructionScript`)