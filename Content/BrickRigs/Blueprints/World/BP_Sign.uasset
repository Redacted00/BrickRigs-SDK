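; BP_Sign is a world Blueprint that lets the player toggle an on-screen widget with the NumPad 5 key.
; Tick polls the first player controller for the key press and feeds a FlipFlop, which alternately creates a new widget in the viewport and removes it.
; Both branches set the mouse cursor visible, so closing the widget leaves the cursor showing.
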(event `self.ReceiveTick`
  (params (DeltaSeconds :type "Float (single-precision)"))
  (if (`PlayerController.WasInputKeyJustPressed` (`GameplayStatics.GetPlayerController` 0) "NumPadFive")
    (`/Engine/EditorBlueprintResources/StandardMacros.FlipFlop`
      (:`A`
        (bind _returnvalue (`|CreateWidget` "/Game/BrickRigs/Blueprints/World/Widget.Widget_C"))
        (`UserWidget.AddToViewport` _returnvalue 0)
        (set `PlayerController.bShowMouseCursor` true (`GameplayStatics.GetPlayerController` 0)))
      (:`B`
        (`Widget.RemoveFromParent` _returnvalue)
        (set `PlayerController.bShowMouseCursor` true (`GameplayStatics.GetPlayerController` 0))))))

(fn `UserConstructionScript`)